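; BP_AudioTriggerBox is a trigger volume that plays a one-time pair of sounds when the player walks into it.
; Box overlap checks for player character 0, prints its name on every such overlap, then passes through a DoOnce that is never reset.
; The configurable SoundToPlay fires at the LocationForAudio component's world position, followed after a short delay by a fixed evil laugh cue at the same spot.
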(event OnComponentBeginOverlap(Box)
  (params (OverlappedComponent :type Primitive%20Component%20Object%20Reference) (OtherActor :type Actor%20Object%20Reference) (OtherComp :type Primitive%20Component%20Object%20Reference) (OtherBodyIndex :type Integer) (bFromSweep :type Boolean) (SweepResult :type Hit%20Result%20Structure%20%28by%20ref%29))
  (bind _locationforaudio (Variables|Default|GetLocationForAudio))
  (bind _returnvalue (Transformation|GetWorldLocation _locationforaudio))
  (if (== OtherActor (Game|GetPlayerCharacter 0))
    (bind _output_get (Variables|Default|SetOther%20Actor OtherActor))
    (Development|PrintString (Utilities|GetDisplayName _output_get))
    (Utilities|FlowControl|DoOnce false
      (:Completed
        (Audio|PlaySoundatLocation (Variables|Default|GetSoundToPlay) _returnvalue "0, 0, 0" 1.0 1.0 0.0 0 0 0 0)
        (Utilities|FlowControl|Delay 4.0)
        (Audio|PlaySoundatLocation "/Game/Assets/Audio/SFX/EvilLaugh_Cue.EvilLaugh_Cue" _returnvalue "0, 0, 0" 1.0 1.0 0.0 0 0 0 0)))))

(fn ConstructionScript)